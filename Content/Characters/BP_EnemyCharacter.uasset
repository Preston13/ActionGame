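; Enemy character Blueprint that runs the BT_Enemy behavior tree on its AI controller at BeginPlay.
; PawnSensing sightings go to DetectPawn along with the player pawn as the target.
; Incoming damage reduces health in StatsComp, whose zero-health delegate triggers HandleDeath.
; Select and deselect events show and hide a lock-on widget for player targeting.
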(event OnSeePawn(PawnSensing)
  (params (Pawn :type Pawn%20Object%20Reference))
  (Class|EnemyCharacter|DetectPawn Pawn (Game|Player|GetPlayerPawn 0)))

(event OnZeroHealthDelegate(StatsComp)
  (Class|EnemyCharacter|HandleDeath))

(event EventBeginPlay
  (AI|RunBehaviorTree (AI|GetAIController self) "/Game/Characters/AI/BT_Enemy.BT_Enemy"))

(event Collision|EventActorBeginOverlap
  (params (OtherActor :type Actor%20Object%20Reference)))

(event EventTick
  (params (DeltaSeconds :type Float%20%28single-precision%29)))

(event Game|Damage|EventAnyDamage
  (params (Damage :type Float%20%28single-precision%29) (DamageType :type Damage%20Type%20Object%20Reference) (InstigatedBy :type Controller%20Object%20Reference) (DamageCauser :type Actor%20Object%20Reference))
  (Class|StatsComponent|ReduceHealth (Variables|Default|GetStatsComp) Damage))

(event EventOnSelect
  (Rendering|SetVisibility (Variables|Default|GetLockonWidget) true false))

(event EventOnDeselect
  (Rendering|SetVisibility (Variables|Default|GetLockonWidget) false false))

(fn ConstructionScript)