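; BP_Boss is a boss character that runs the BT_Boss behavior tree on its AI controller at BeginPlay.
; Incoming damage is passed to StatsComp to reduce health, and selection events show or hide its lock-on widget.
; PawnSensing forwards each seen pawn to DetectPawn along with the player pawn as the target to match.
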(event OnSeePawn(PawnSensing)
  (params (Pawn :type Pawn%20Object%20Reference))
  (Class|BossCharacter|DetectPawn Pawn (Game|Player|GetPlayerPawn 0)))

(event EventBeginPlay
  (AI|RunBehaviorTree (AI|GetAIController self) "/Game/Characters/AI/BT_Boss.BT_Boss"))

(event EventTick
  (params (DeltaSeconds :type Float%20%28single-precision%29)))

(event EventOnSelect
  (Rendering|SetVisibility (Variables|Default|GetLockonWidget) true false))

(event EventOnDeselect
  (Rendering|SetVisibility (Variables|Default|GetLockonWidget) false false))

(event Game|Damage|EventAnyDamage
  (params (Damage :type Float%20%28single-precision%29) (DamageType :type Damage%20Type%20Object%20Reference) (InstigatedBy :type Controller%20Object%20Reference) (DamageCauser :type Actor%20Object%20Reference))
  (Class|StatsComponent|ReduceHealth (Variables|Default|GetStatsComp) Damage))

(fn ConstructionScript)