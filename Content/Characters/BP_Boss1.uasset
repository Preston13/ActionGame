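; Boss enemy character that runs the BT_Boss behavior tree on its AI controller and shows a lock-on widget when selected.
; Sighting a pawn calls DetectPawn with the player pawn as target and creates the boss health bar once, re-armed after combat ends.
; Damage goes to the stats component, whose delegates update the health bar, remove it on leaving combat, and trigger death handling at zero health.
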(event OnSeePawn(PawnSensing)
  (params (Pawn :type Pawn%20Object%20Reference))
  (Class|BossCharacter|DetectPawn Pawn (Game|Player|GetPlayerPawn 0))
  (Utilities|FlowControl|DoOnce false
    (:Completed
      (bind _returnvalue (UserInterface|CreateWidget "/Game/UI/WBP_Boss.WBP_Boss_C"))
      (bind _output_get (Variables|Default|SetBossWidget _returnvalue))
      (UserInterface|Viewport|AddtoViewport _output_get 0)
      (Default|SetHealth (Variables|Default|GetBossWidget) (Class|StatsComponent|GetStatPercentage (Variables|Default|GetStatsComp) "Health" "MaxHealth")))))

(event OnHealthPercentUpdateDelegate(StatsComp)
  (params (Percentage :type Float%20%28single-precision%29))
  (Default|SetHealth (Variables|Default|GetBossWidget) Percentage))

(event OnZeroHealthDelegate(StatsComp)
  (Class|BossCharacter|HandleDeath)
  (Widget|RemovefromParent (Variables|Default|GetBossWidget)))

(event OnLeaveCombatDelegate(StatsComp)
  (Widget|RemovefromParent (Variables|Default|GetBossWidget))
  (Utilities|FlowControl|DoOnce false) ; enters at Reset
)

(event EventBeginPlay
  (AI|RunBehaviorTree (AI|GetAIController self) "/Game/Characters/AI/BT_Boss.BT_Boss"))

(event EventTick
  (params (DeltaSeconds :type Float%20%28single-precision%29)))

(event EventOnSelect
  (Rendering|SetVisibility (Variables|Default|GetLockonWidget) true false))

(event EventOnDeselect
  (Rendering|SetVisibility (Variables|Default|GetLockonWidget) false false))

(event Game|Damage|EventAnyDamage
  (params (Damage :type Float%20%28single-precision%29) (DamageType :type Damage%20Type%20Object%20Reference) (InstigatedBy :type Controller%20Object%20Reference) (DamageCauser :type Actor%20Object%20Reference))
  (Class|StatsComponent|ReduceHealth (Variables|Default|GetStatsComp) Damage))

(fn ConstructionScript)